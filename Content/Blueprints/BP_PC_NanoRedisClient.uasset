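; Player controller test harness for a NanoRedis client, exercising Redis commands from key presses and printing results on screen.
; BeginPlay creates a client for a hard-coded server and password, then pings it.
; Z and X send raw GET and INCR commands, while F batches commands through a reusable pipeline.
; G runs a reusable transaction, chaining queue callbacks into a commit that fires even if the last queue fails, then prints results by type.
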(event Custom|OnPingDone
  (params (Ok :type Boolean) (Err :type String) (Value :type Reply%20Value%20Structure%20%28by%20ref%29))
  (if Ok
    (Development|PrintString (.Status (Utilities|Struct|BreakReplyValue Value)))
    (else
      (Development|PrintString Err))))

(event Custom|OnINCRPerson
  (params (Ok :type Boolean) (Err :type String) (Value :type Reply%20Value%20Structure%20%28by%20ref%29))
  (if Ok
    (Development|PrintString (Utilities|String|ToString(Integer) (.Integer (Utilities|Struct|BreakReplyValue Value))) true true "(R=1.000000,G=0.215023,B=0.167248,A=1.000000)" 5.0)
    (else
      (Development|PrintString Err))))

(event Custom|OnGetPerson
  (params (Ok :type Boolean) (Err :type String) (Value :type Reply%20Value%20Structure%20%28by%20ref%29))
  (if Ok
    (Development|PrintString (.String (Utilities|Struct|BreakReplyValue Value)) true true "(R=1.000000,G=0.215023,B=0.167248,A=1.000000)" 5.0)
    (else
      (Development|PrintString Err))))

(event Custom|OnCommit
  (params (Ok :type Boolean) (Err :type String) (Values :type Array%20of%20Reply%20Value%20Structures))
  (if Ok
    (for _array_element Values
      (switch Utilities|FlowControl|Switch|SwitchonEReplyValueType (.Type (Utilities|Struct|BreakReplyValue _array_element))
        (:EInt
          (Development|PrintString (Utilities|String|ToString(Integer) (.Integer (Utilities|Struct|BreakReplyValue _array_element)))))
        (:EString
          (Development|PrintString (.String (Utilities|Struct|BreakReplyValue _array_element))))
        (:EList
          (for _array_element_2 (.List (Utilities|Struct|BreakReplyValue _array_element))
            (Development|PrintString (.String (Utilities|Struct|BreakListReplyValue _array_element_2)))))
        (:EStatus
          (Development|PrintString (.Status (Utilities|Struct|BreakReplyValue _array_element))))))
    (else
      (Development|PrintString Err))))

(event Custom|OnStart
  (params (Ok :type Boolean) (Err :type String) (Value :type Reply%20Value%20Structure%20%28by%20ref%29))
  (if Ok
    (Class|RedisTransaction|Queue (Variables|Default|GetRedis%20Transaction) "LRANGE name 0 -1" (delegate Custom|OnLRange))
    (else
      (Development|PrintString Err))))

(event Custom|OnLRange
  (params (Ok :type Boolean) (Err :type String) (Value :type Reply%20Value%20Structure%20%28by%20ref%29))
  (if Ok
    (Class|RedisTransaction|Queue (Variables|Default|GetRedis%20Transaction) "INCR person" (delegate Custom|OnINCR))
    (else
      (Development|PrintString Err))))

(event Custom|OnCommitAll
  (params (Ok :type Boolean) (Err :type String) (Value :type Reply%20Value%20Structure%20%28by%20ref%29))
  (if Ok
    (for _array_element (.List (Utilities|Struct|BreakReplyValue Value))
      (switch Utilities|FlowControl|Switch|SwitchonEReplyValueType (.Type (Utilities|Struct|BreakListReplyValue _array_element))
        (:EInt
          (Development|PrintString (Utilities|String|ToString(Integer) (.Integer (Utilities|Struct|BreakListReplyValue _array_element)))))
        (:EString
          (Development|PrintString (.String (Utilities|Struct|BreakListReplyValue _array_element))))
        (:EList
          (for _array_element_2 (.List (Utilities|Struct|BreakListReplyValue _array_element))
            (Development|PrintString _array_element_2)))
        (:EStatus
          (Development|PrintString (.Status (Utilities|Struct|BreakListReplyValue _array_element))))))
    (else
      (Development|PrintString Err))))

(event Custom|OnINCR
  (params (Ok :type Boolean) (Err :type String) (Value :type Reply%20Value%20Structure%20%28by%20ref%29))
  (if Ok
    (Class|RedisTransaction|Queue (Variables|Default|GetRedis%20Transaction) "GET person" (delegate Custom|OnQueue))
    (else
      (Development|PrintString Err))))

(event Custom|OnQueue
  (params (Ok :type Boolean) (Err :type String) (Value :type Reply%20Value%20Structure%20%28by%20ref%29))
  (if true
    (Class|RedisTransaction|Commit (Variables|Default|GetRedis%20Transaction) (delegate Custom|OnCommitAll))
    (else
      (Development|PrintString Err))))

(event EventBeginPlay
  (bind _returnvalue (Class|RedisClient|NewRedisClient 3 "192.168.3.95" 6379 "12345678"))
  (Variables|Default|SetRedis%20Client _returnvalue)
  (Class|RedisClient|Ping (Variables|Default|GetRedis%20Client) (delegate Custom|OnPingDone)))

(event Input|KeyboardEvents|G
  (params (Key :type Key%20Structure :default "None"))
  (:Pressed
    (Utilities|IsValid (Variables|Default|GetRedis%20Client)
      (:Is%20Valid
        (Utilities|IsValid (Variables|Default|GetRedis%20Transaction)
          (:Is%20Valid
            _)
          (:Is%20Not%20Valid
            (bind _returnvalue (Class|RedisClient|NewTransaction (Variables|Default|GetRedis%20Client)))
            (Variables|Default|SetRedis%20Transaction _returnvalue)))
        (Class|RedisTransaction|Start (Variables|Default|GetRedis%20Transaction) (delegate Custom|OnStart))))))

(event Input|KeyboardEvents|Z
  (params (Key :type Key%20Structure :default "None"))
  (:Pressed
    (Utilities|IsValid (Variables|Default|GetRedis%20Client)
      (:Is%20Valid
        (Class|RedisClient|Raw (Variables|Default|GetRedis%20Client) "GET person" (delegate Custom|OnGetPerson))))))

(event Input|KeyboardEvents|X
  (params (Key :type Key%20Structure :default "None"))
  (:Pressed
    (Utilities|IsValid (Variables|Default|GetRedis%20Client)
      (:Is%20Valid
        (Class|RedisClient|Raw (Variables|Default|GetRedis%20Client) "INCR person" (delegate Custom|OnINCRPerson))))))

(event Input|KeyboardEvents|F
  (params (Key :type Key%20Structure :default "None"))
  (:Pressed
    (Utilities|IsValid (Variables|Default|GetRedis%20Client)
      (:Is%20Valid
        (Utilities|IsValid (Variables|Default|GetRedis%20Pipeline)
          (:Is%20Valid
            _)
          (:Is%20Not%20Valid
            (bind _returnvalue (Class|RedisClient|NewPipeline (Variables|Default|GetRedis%20Client)))
            (Variables|Default|SetRedis%20Pipeline _returnvalue)))
        (Class|RedisPipeline|Start (Variables|Default|GetRedis%20Pipeline))
        (Class|RedisPipeline|Exec (Variables|Default|GetRedis%20Pipeline) "LRANGE name 0 -1")
        (Class|RedisPipeline|Exec (Variables|Default|GetRedis%20Pipeline) "INCR person")
        (Class|RedisPipeline|Exec (Variables|Default|GetRedis%20Pipeline) "GET person")
        (Class|RedisPipeline|Commit (Variables|Default|GetRedis%20Pipeline) (delegate Custom|OnCommit))))))

(fn ConstructionScript)